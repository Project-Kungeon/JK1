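; BP_LobbyPawn is the player pawn for the lobby, pairing the lobby UI with basic movement input.
; On BeginPlay it adds the IMC_JK1 Enhanced Input mapping context, creates WBP_LobbyWidget on the viewport and shows the mouse cursor.
; IA_Move feeds AddMovementInput along the control rotation's forward (X) and right (Y) vectors.
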(event `self.ReceiveBeginPlay`
  (`EnhancedInputSubsystemInterface.AddMappingContext` (pcsubsystem `EnhancedInputLocalPlayerSubsystem` (`GameplayStatics.GetPlayerController` 0)) "/Game/Input/IMC_JK1.IMC_JK1" 0 (struct))
  (bind _returnvalue (`|CreateWidget` "/Game/Blueprints/Widget/Lobby/WBP_LobbyWidget.WBP_LobbyWidget_C"))
  (`UserWidget.AddToViewport` _returnvalue 0)
  (set `PlayerController.bShowMouseCursor` true (`GameplayStatics.GetPlayerController` 0)))

(event `EnhancedInput|/Game/Input/Action/IA_Move`
  (params (ActionValue :type "Vector2D Structure") (ElapsedSeconds :type "Float (double-precision)") (TriggeredSeconds :type "Float (double-precision)") (InputAction :type "InputAction Object Reference" :default "/Game/Input/Action/IA_Move.IA_Move"))
  (bind _returnvalue (`self.GetControlRotation`))
  (:`Triggered`
    (`self.AddMovementInput` (`KismetMathLibrary.GetForwardVector` _returnvalue) ActionValue_X)
    (`self.AddMovementInput` (`KismetMathLibrary.GetRightVector` _returnvalue) ActionValue_Y)))

(fn `UserConstructionScript`)